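; Portal actor that shows a live view from its linked TargetRoom portal and teleports the FirstPersonCharacter to that portal's Arrow on hit.
; Shortly after BeginPlay, it renders the target's SceneCapture2D to a runtime render target shown through a dynamic Portal_Mat instance.
; Each Tick slides that capture along the target Arrow's forward axis by player camera distance, without rotating it.
; Automatic pairing code is disconnected, leaving SetTargetPortal empty.
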(event EventBeginPlay
  (Variables|Default|SetoldRotation (Transformation|GetWorldRotation (Variables|Default|GetSceneCapture2D)))
  (Utilities|FlowControl|Delay 0.2)
  (CallFunction|SetPortalView))

(event Collision|EventActorBeginOverlap
  (params (OtherActor :type Actor%20Object%20Reference)))

(event EventTick
  (params (DeltaSeconds :type Float%20%28single-precision%29))
  (CallFunction|UpdateSceneCapture))

(event Collision|EventHit
  (params (MyComp :type Primitive%20Component%20Object%20Reference) (Other :type Actor%20Object%20Reference) (OtherComp :type Primitive%20Component%20Object%20Reference) (bSelfMoved :type Boolean) (HitLocation :type Vector :default "0, 0, 0") (HitNormal :type Vector :default "0, 0, 0") (NormalImpulse :type Vector :default "0, 0, 0") (Hit :type Hit%20Result%20Structure%20%28by%20ref%29))
  (bind _targetroom (Variables|Default|GettargetRoom))
  (bind _arrow (Variables|Portal_BP_C|GetArrow _targetroom))
  (bind _asfirst_person_character (Utilities|Casting|CastToFirstPersonCharacter Other))
  (Utilities|IsValid _targetroom
    (:Is%20Valid
      (Default|PlayerTeleport _asfirst_person_character (Transformation|GetWorldLocation _arrow) (Transformation|GetWorldRotation _arrow)))))

(fn ConstructionScript)

(fn GetAllPortals
  (bind _outactors (Actor|GetAllActorsOfClass "Portal_BP_C"))
  (Variables|Default|Setportals _outactors)
  (return))

(fn SetTargetPortal)

(fn SetPortalView
  (bind _targetroom (Variables|Default|GettargetRoom))
  (Utilities|IsValid _targetroom
    (:Is%20Valid
      (Rendering|Material|SetMaterial (Variables|Default|GetPortal) 0 (CallFunction|GetSceneCaptureMaterial _targetroom)))))

(fn UpdateSceneCapture
  (bind _targetroom (Variables|Default|GettargetRoom))
  (bind _arrow (Variables|Portal_BP_C|GetArrow _targetroom))
  (bind _returnvalue (Math|Vector|GetForwardVector _arrow))
  (Transformation|SetWorldLocation (Variables|Portal_BP_C|GetSceneCapture2D _targetroom) (+ (* (* _returnvalue -1.0) (Math|Conversions|ToVector(Float) (CallFunction|DistanceBetweenPlayer))) (Transformation|GetWorldLocation _arrow) (* _returnvalue 3.5e+02)) false false))

(fn SetPortalViewLocationandRotation
  (params (NewLocation :type Vector) (NewRotation :type Rotator))
  (Transformation|SetWorldRotation (Variables|Default|GetSceneCapture2D) NewRotation false false))

(fn PlayerCameraTransform
  (return (Variables|/Script/Engine.PlayerCameraManager|GetTransformComponent (Variables|/Script/Engine.PlayerController|GetPlayerCameraManager (Game|GetPlayerController 0)))))

(fn DistanceBetweenPlayer
  (return (Math|Vector|VectorLength (- (Transformation|GetWorldLocation (CallFunction|PlayerCameraTransform)) (Transformation|GetWorldLocation (Variables|Default|GetArrow))))))

(fn NumberMatching
  (params (length :type Integer))
  (if (== (Math|Integer|%(Integer) length 2) 0)
    _))

(fn GetSceneCaptureMaterial
  (params (TargetRoom :type Portal%20BP%20Object%20Reference))
  (bind _returnvalue (Rendering|CreateRenderTarget2D 1980 1080 "RTF_RGBA16f"))
  (bind _output_get (Variables|/Script/Engine.SceneCaptureComponent2D|SetTextureTarget (Variables|Portal_BP_C|GetSceneCapture2D TargetRoom) _returnvalue))
  (bind _returnvalue_2 (Rendering|Material|CreateDynamicMaterialInstance "/Game/Blueprints/Portal/Portal_Mat.Portal_Mat" (Utilities|String|StringToName (Utilities|GetDisplayName self)) :!class /Script/Engine.KismetMaterialLibrary))
  (Rendering|Material|SetTextureParameterValue _returnvalue_2 "View" _output_get)
  (return _returnvalue_2))